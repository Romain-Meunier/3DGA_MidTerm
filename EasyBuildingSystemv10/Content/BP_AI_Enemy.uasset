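; Enemy AI actor that turns toward and attacks a player character of the Ue4ASP_Character class when it sees one.
; PawnSensing's See Pawn event snaps its rotation to face the target, then spawns BP_Projectile at SpawnProjectileLocation.
; Damage is applied directly to the target at the moment of firing, independent of any projectile hit.
; A CanAttack flag and a short Delay throttle the attack rate.
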(event OnSeePawn(PawnSensing)
  (params (Pawn :type Pawn%20Object%20Reference))
  (bind _asue_4asp_character (Utilities|Casting|CastToUe4ASP_Character Pawn))
  (Transformation|SetActorRotation (Math|Rotator|FindRelativeLookatRotation (Math|Conversions|ToTransform(Vector) (Transformation|GetActorLocation)) (Transformation|GetActorLocation _asue_4asp_character)))
  (if (Variables|Default|GetCanAttack?)
    (Game|SpawnActorfromClass "/Game/BP_Projectile.BP_Projectile_C" (Transformation|GetWorldTransform (Variables|Default|GetSpawnProjectileLocation)) "Undefined" 0 0)
    (Game|Damage|ApplyDamage _asue_4asp_character 1.0 0 0)
    (Variables|Default|SetCanAttack? false)
    (Utilities|FlowControl|Delay 0.5)
    (Variables|Default|SetCanAttack? true)))

(event EventBeginPlay)

(event Collision|EventActorBeginOverlap
  (params (OtherActor :type Actor%20Object%20Reference)))

(event EventTick
  (params (DeltaSeconds :type Float%20%28single-precision%29)))

(fn ConstructionScript)